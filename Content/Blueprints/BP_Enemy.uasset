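; BP_Enemy is an enemy actor whose Box component wanders aimlessly from BeginPlay onward.
; It loops endlessly through two latent MoveComponentTo steps separated by zero-length delays.
; The first eases the Box forward by a random distance over a random duration, and the second turns it by a random yaw over a fixed time.
; It has no player detection, collision response or construction logic.
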(event `self.ReceiveBeginPlay`
  (bind _returnvalue (`KismetMathLibrary.RandomFloatInRange` 50.0 400.0))
  (bind _box (`self.Box`))
  (bind _box_2 (`self.Box`))
  (`KismetSystemLibrary.MoveComponentTo` _box (+ (`SceneComponent.RelativeLocation` _box) (* (`SceneComponent.GetForwardVector` _box) _returnvalue)) (`SceneComponent.RelativeRotation` _box) true true (/ _returnvalue 100.0) :!label _label)
  (`KismetSystemLibrary.Delay` 0.0)
  (`KismetSystemLibrary.MoveComponentTo` _box_2 (`SceneComponent.RelativeLocation` _box_2) (`KismetMathLibrary.ComposeRotators` (`SceneComponent.RelativeRotation` _box_2) (`KismetMathLibrary.MakeRotator` 0.0 0.0 (`KismetMathLibrary.RandomFloatInRange` 90.0 270.0))) false false 1.0 true)
  (`KismetSystemLibrary.Delay` 0.0)
  (goto _label))

(fn `UserConstructionScript`)