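; DamageBox is a damage zone that hurts a ThirdPersonCharacter periodically while it overlaps the DamageBox component.
; Begin overlap stores the character and starts a looping one-second timer, whose event applies fixed damage and prints the result.
; End overlap clears the stored timer handle, stopping the damage.
; Only one character reference and one timer handle are stored, so the first tick lands a second after entry.
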(event `self.damageBox.OnComponentBeginOverlap`
  (params (OverlappedComponent :type "PrimitiveComponent Object Reference") (OtherActor :type "Actor Object Reference") (OtherComp :type "PrimitiveComponent Object Reference") (OtherBodyIndex :type Integer) (bFromSweep :type Boolean) (SweepResult :type "HitResult Structure (by ref)"))
  (bind _asthird_person_character (cast `/Game/ThirdPersonBP/Blueprints/ThirdPersonCharacter` OtherActor))
  (set `self.As Third Person Character` _asthird_person_character)
  (bind _returnvalue (`KismetSystemLibrary.K2_SetTimerDelegate` (delegate `add damagae`) 1.0 true))
  (set `self.timer_ref` _returnvalue))

(event `add damagae`
  (bind _returnvalue (`GameplayStatics.ApplyDamage` (`self.As Third Person Character`) 9.0))
  (`KismetSystemLibrary.PrintString` (`KismetStringLibrary.Conv_DoubleToString` _returnvalue)))

(event `self.damageBox.OnComponentEndOverlap`
  (params (OverlappedComponent :type "PrimitiveComponent Object Reference") (OtherActor :type "Actor Object Reference") (OtherComp :type "PrimitiveComponent Object Reference") (OtherBodyIndex :type Integer))
  (cast `/Game/ThirdPersonBP/Blueprints/ThirdPersonCharacter` OtherActor)
  (`KismetSystemLibrary.K2_ClearAndInvalidateTimerHandle` (`self.timer_ref`)))

(fn `UserConstructionScript`)